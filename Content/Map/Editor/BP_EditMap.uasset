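; Hex map actor for the map editor that builds a grid of BP_Hex tiles and previews a path across it.
; BeginPlay spawns offset-column hexes into a coordinate-keyed map and hands it to BP_EditorController.
; A hand-written A* links tiles through PreviousHex, penalises height steps of two or more, and marks the path between two fixed test cells.
; RefreshPath resets every hex and reruns that search; LoadMap is an empty stub.
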(event Custom|LoadMap)

(event Custom|RefreshPath
  ;[1 1 1] Refresh path after changes
  (for _array_element (Variables|Default|GetHexIndexes)
    (Default|RefreshHex (.Value (Utilities|Map|Find (Variables|Default|GetHexArray) _array_element))))
  ;[1 1 1] AStar
  (bind _path (CallFunction|FindPath "(X=0.000000,Y=0.000000)" "(X=10.000000,Y=10.000000)" (Variables|Default|GetHexArray)))
  (for _array_element_2 _path
    (Default|HexPath (.Value (Utilities|Map|Find (Variables|Default|GetHexArray) _array_element_2)))))

(event EventBeginPlay
  ;[1 1 1] Map generation
  (for _index (range 0 (Variables|MapGeneration|GetXCount))
    (Variables|MapGeneration|SetX_L _index)
    (for _index_2 (range 0 (Variables|MapGeneration|GetYCount))
      (Variables|MapGeneration|SetY_L _index_2)
      (bind _output_get (Variables|MapGeneration|SetHexPosition (Math|Vector|SelectVector (CallFunction|Diagonal1Pos) (CallFunction|Diagonal2Pos) (== (Math|Integer|%(Integer) (Variables|MapGeneration|GetX_L) 2) 0))))
      (bind _returnvalue (Game|SpawnActorfromClass "/Game/Map/Hexes/BP_Hex.BP_Hex_C" (Math|Transform|MakeTransform _output_get "0, 0, 0" "1,1,1") "Undefined" 0 (Math|Vector2D|MakeVector2D (Math|Conversions|ToFloat(Integer) (Variables|MapGeneration|GetX_L)) (Math|Conversions|ToFloat(Integer) (Variables|MapGeneration|GetY_L))) 0))
      (Utilities|Map|Add (Variables|Default|GetHexArray) (Variables|/Game/Map/Hexes/BP_Hex.BP_Hex_C|GetIndexXY _returnvalue) _returnvalue)
      (Utilities|Array|AddUnique (Variables|Default|GetHexIndexes) (Variables|/Game/Map/Hexes/BP_Hex.BP_Hex_C|GetIndexXY _returnvalue))))
  (bind _asbp_editor_controller (Utilities|Casting|CastToBP_EditorController (Game|GetPlayerController 0)))
  (Variables|/Game/Map/ModeCameraController/BP_EditorController.BP_EditorController_C|SetHexMap _asbp_editor_controller (Variables|Default|GetHexArray))
  (Variables|/Game/Map/ModeCameraController/BP_EditorController.BP_EditorController_C|SetEditingMap _asbp_editor_controller self)
  ;[1 1 1] AStar
  (bind _path (CallFunction|FindPath "(X=0.000000,Y=0.000000)" "(X=10.000000,Y=10.000000)" (Variables|Default|GetHexArray)))
  (for _array_element _path
    (Default|HexPath (.Value (Utilities|Map|Find (Variables|Default|GetHexArray) _array_element)))))

(fn ConstructionScript)

(fn Hex1Position
  (bind _returnvalue (Transformation|GetActorLocation))
  (return (Math|Vector|MakeVector (+ (* (Variables|MapGeneration|GetX_L) (* (Variables|MapGeneration|GetHexMediana) 2.0)) (.x _returnvalue)) (+ (.y _returnvalue) (* (Variables|MapGeneration|GetY_L) (* (Utilities|HexR) 1.5))) (.z _returnvalue))))

(fn Hex2Position
  (bind _returnvalue (Transformation|GetActorLocation))
  (return (Math|Vector|MakeVector (+ (.x _returnvalue) (- (* (Variables|MapGeneration|GetX_L) (* (Variables|MapGeneration|GetHexMediana) 2.0)) (Variables|MapGeneration|GetHexMediana))) (+ (* (Variables|MapGeneration|GetY_L) (* (Utilities|HexR) 1.5)) (.y _returnvalue)) (.z _returnvalue))))

(fn GetNeighbours
  (params (Hex :type Vector%202D%20Structure))
  (LocalVariables|Setl_Hex Hex)
  (bind _output_get (LocalVariables|SetPossibles_L (select (or (== (Math|Float|%(Float) (.x (LocalVariables|Getl_Hex)) 2.0) 0.0) (== (.x (LocalVariables|Getl_Hex)) 0.0)) (Utilities|Array|MakeArray "(X=1.000000,Y=0.000000)" "(X=1.000000,Y=-1.000000)" "(X=0.000000,Y=-1.000000)" "(X=-1.000000,Y=-1.000000)" "(X=-1.000000,Y=0.000000)" "(X=0.000000,Y=1.000000)") (Utilities|Array|MakeArray "(X=1.000000,Y=1.000000)" "(X=1.000000,Y=0.000000)" "(X=0.000000,Y=-1.000000)" "(X=-1.000000,Y=0.000000)" "(X=-1.000000,Y=1.000000)" "(X=0.000000,Y=1.000000)"))))
  (for (_array_element _array_index) _output_get
    (Utilities|Array|SetArrayElem (LocalVariables|GetPossibles_L) _array_index (+ _array_element (LocalVariables|Getl_Hex))))
  (return (LocalVariables|GetPossibles_L)))

(fn GetCostBetween
  (params (CurrentHex :type Vector%202D%20Structure) (TargetHex :type Vector%202D%20Structure))
  (bind _returnvalue (- CurrentHex TargetHex))
  (return (Math|Float|Round (+ (Math|Float|Absolute(Float) (.x _returnvalue)) (Math|Float|Absolute(Float) (.y _returnvalue))))))

(fn RetracePath
  (params (TargetHex :type Vector%202D%20Structure) (StartHex :type Vector%202D%20Structure) (HexMap :type Map%20of%20Vector%202D%20Structures%20to%20Objects))
  (bind _output_get (LocalVariables|Setl_CurrentHex TargetHex))
  (LocalVariables|Setl_HexMap HexMap)
  (while (Math|Vector|NotEqual(Vector) _output_get StartHex 0.0001)
    (Utilities|Array|AddUnique (LocalVariables|Getl_invertedPath) (LocalVariables|Getl_CurrentHex))
    (LocalVariables|Setl_CurrentHex (Variables|/Game/Map/Hexes/BP_Hex.BP_Hex_C|GetPreviousHex (.Value (Utilities|Map|Find (LocalVariables|Getl_HexMap) (LocalVariables|Getl_CurrentHex))))))
  (bind _arrayelement (Utilities|Array|ReverseforEachLoop (LocalVariables|Getl_invertedPath))
    (:LoopBody
      (Utilities|Array|AddUnique (LocalVariables|Getl_setPath) _arrayelement))
    (:Completed
      (return (LocalVariables|Getl_setPath)))))

(fn FindPath
  (params (Start :type Vector%202D%20Structure) (Target :type Vector%202D%20Structure) (HexMap :type Map%20of%20Vector%202D%20Structures%20to%20Objects))
  (LocalVariables|Setl_Start Start)
  (LocalVariables|Setl_Target Target)
  (LocalVariables|Setl_HexMap HexMap)
  (bind _output_get (LocalVariables|Setl_CurrentHex (LocalVariables|Getl_Start)))
  (Utilities|Array|AddUnique (LocalVariables|Getl_OpenSet) _output_get)
  (while (> (Utilities|Array|Length (LocalVariables|Getl_OpenSet)) 0)
    (LocalVariables|Setl_OpenSetClosest (Utilities|Array|Get(acopy) (LocalVariables|Getl_OpenSet)))
    (for _array_element (LocalVariables|Getl_OpenSet)
      (bind _output_get_2 (LocalVariables|Setl_CheckNeighbour _array_element))
      (if (< (Variables|/Game/Map/Hexes/BP_Hex.BP_Hex_C|GetHexCost (.Value (Utilities|Map|Find (LocalVariables|Getl_HexMap) _output_get_2))) (Variables|/Game/Map/Hexes/BP_Hex.BP_Hex_C|GetHexCost (.Value (Utilities|Map|Find (LocalVariables|Getl_HexMap) (LocalVariables|Getl_OpenSetClosest)))))
        (LocalVariables|Setl_OpenSetClosest (LocalVariables|Getl_CheckNeighbour))))
    (if (not (Math|Vector|Equal(Vector) (LocalVariables|Getl_OpenSetClosest) (LocalVariables|Getl_Target) 0.0001))
      (Utilities|Array|RemoveItem (LocalVariables|Getl_OpenSet) (LocalVariables|Getl_CurrentHex))
      (Utilities|Array|AddUnique (LocalVariables|Getl_ClosedSet) (LocalVariables|Getl_CurrentHex))
      (bind _output_get_3 (LocalVariables|Setl_CurrentHex (LocalVariables|Getl_OpenSetClosest)))
      (for _array_element_2 (CallFunction|GetNeighbours _output_get_3)
        (LocalVariables|Setl_CurrentNeighbour _array_element_2)
        (if (and (not (Utilities|Array|ContainsItem (LocalVariables|Getl_ClosedSet) _array_element_2)) (Utilities|Map|Contains (LocalVariables|Getl_HexMap) (LocalVariables|Getl_CurrentNeighbour)))
          (if (not (Utilities|Array|ContainsItem (LocalVariables|Getl_OpenSet) (LocalVariables|Getl_CurrentNeighbour)))
            (Utilities|Array|AddUnique (LocalVariables|Getl_OpenSet) (LocalVariables|Getl_CurrentNeighbour))
            (Variables|/Game/Map/Hexes/BP_Hex.BP_Hex_C|SetPreviousHex (.Value (Utilities|Map|Find (LocalVariables|Getl_HexMap) (LocalVariables|Getl_CurrentNeighbour))) (LocalVariables|Getl_CurrentHex))
            (Variables|/Game/Map/Hexes/BP_Hex.BP_Hex_C|SetGCost (.Value (Utilities|Map|Find (LocalVariables|Getl_HexMap) (LocalVariables|Getl_CurrentNeighbour))) (CallFunction|GCostCalculate (LocalVariables|Getl_CurrentHex) (LocalVariables|Getl_CurrentNeighbour) (LocalVariables|Getl_HexMap)))
            (Variables|/Game/Map/Hexes/BP_Hex.BP_Hex_C|SetHCost (.Value (Utilities|Map|Find (LocalVariables|Getl_HexMap) (LocalVariables|Getl_CurrentNeighbour))) (CallFunction|GetCostBetween (LocalVariables|Getl_CurrentNeighbour) (LocalVariables|Getl_Target)))
            (Default|HexCostCalculate (.Value (Utilities|Map|Find (LocalVariables|Getl_HexMap) (LocalVariables|Getl_CurrentNeighbour))))
            (elif (< (CallFunction|GCostRecalculate (LocalVariables|Getl_CurrentHex) (LocalVariables|Getl_CurrentNeighbour) (LocalVariables|Getl_HexMap)) (Variables|/Game/Map/Hexes/BP_Hex.BP_Hex_C|GetGCost (.Value (Utilities|Map|Find (LocalVariables|Getl_HexMap) (LocalVariables|Getl_CurrentNeighbour)))))
              (Variables|/Game/Map/Hexes/BP_Hex.BP_Hex_C|SetPreviousHex (.Value (Utilities|Map|Find (LocalVariables|Getl_HexMap) (LocalVariables|Getl_CurrentNeighbour))) (LocalVariables|Getl_CurrentHex))
              (Variables|/Game/Map/Hexes/BP_Hex.BP_Hex_C|SetGCost (.Value (Utilities|Map|Find (LocalVariables|Getl_HexMap) (LocalVariables|Getl_CurrentNeighbour))) (CallFunction|GCostRecalculate (LocalVariables|Getl_CurrentHex) (LocalVariables|Getl_CurrentNeighbour) (LocalVariables|Getl_HexMap)))
              (Default|HexCostCalculate (.Value (Utilities|Map|Find (LocalVariables|Getl_HexMap) (LocalVariables|Getl_CurrentNeighbour))))
              (if (< (Variables|/Game/Map/Hexes/BP_Hex.BP_Hex_C|GetHexCost (.Value (Utilities|Map|Find (LocalVariables|Getl_HexMap) (LocalVariables|Getl_CurrentNeighbour)))) (Variables|/Game/Map/Hexes/BP_Hex.BP_Hex_C|GetHexCost (.Value (Utilities|Map|Find (LocalVariables|Getl_HexMap) (LocalVariables|Getl_OpenSetClosest)))))
                (LocalVariables|Setl_OpenSetClosest (LocalVariables|Getl_CurrentNeighbour)))))))
      (else
        (return (CallFunction|RetracePath (LocalVariables|Getl_Target) (LocalVariables|Getl_Start) (LocalVariables|Getl_HexMap)) (LocalVariables|Getl_OpenSet) (LocalVariables|Getl_ClosedSet))))))

(fn Diagonal2Pos
  (bind _returnvalue (Transformation|GetActorLocation))
  (return (Math|Vector|MakeVector (+ (.x _returnvalue) (* (Variables|MapGeneration|GetX_L) (* (Utilities|HexR) 1.5))) (+ (+ (* (Variables|MapGeneration|GetY_L) (* (Variables|MapGeneration|GetHexMediana) 2.0)) (Variables|MapGeneration|GetHexMediana)) (.y _returnvalue)) (.z _returnvalue))))

(fn Diagonal1Pos
  (bind _returnvalue (Transformation|GetActorLocation))
  (return (Math|Vector|MakeVector (+ (.x _returnvalue) (* (Variables|MapGeneration|GetX_L) (* (Utilities|HexR) 1.5))) (+ (* (Variables|MapGeneration|GetY_L) (* (Variables|MapGeneration|GetHexMediana) 2.0)) (.y _returnvalue)) (.z _returnvalue))))

(fn GetHeightDifference
  (params (Hex1 :type Vector%202D%20Structure) (Hex2 :type Vector%202D%20Structure))
  (bind _hexarray (Variables|Default|GetHexArray))
  (return (Math|Integer|Absolute(Integer) (- (Variables|/Game/Map/Hexes/BP_Hex.BP_Hex_C|GetHeight (.Value (Utilities|Map|Find _hexarray Hex1))) (Variables|/Game/Map/Hexes/BP_Hex.BP_Hex_C|GetHeight (.Value (Utilities|Map|Find _hexarray Hex2)))))))

(fn GCostCalculate
  (params (CurrentHex :type Vector%202D%20Structure) (CurrentNeighbour :type Vector%202D%20Structure) (HexMap :type Map%20of%20Vector%202D%20Structures%20to%20Objects))
  (bind _output_get (LocalVariables|Setl_hexmap HexMap))
  (return (+ (Variables|/Game/Map/Hexes/BP_Hex.BP_Hex_C|GetGCost (.Value (Utilities|Map|Find _output_get CurrentNeighbour))) (Math|Integer|SelectInt (Variables|/Game/Map/Hexes/BP_Hex.BP_Hex_C|GetGCost (.Value (Utilities|Map|Find _output_get CurrentHex))) 100 (< (CallFunction|GetHeightDifference CurrentHex CurrentNeighbour) 2)))))

(fn GCostRecalculate
  (params (CurrentHex :type Vector%202D%20Structure) (CurrentNeighbour :type Vector%202D%20Structure) (HexMap :type Map%20of%20Vector%202D%20Structures%20to%20Objects))
  (bind _output_get (LocalVariables|Setl_HexMap HexMap))
  (return (+ (Variables|/Game/Map/Hexes/BP_Hex.BP_Hex_C|GetGCost (.Value (Utilities|Map|Find _output_get CurrentHex))) (Math|Integer|SelectInt 1 100 (< (CallFunction|GetHeightDifference CurrentHex CurrentNeighbour) 2)))))