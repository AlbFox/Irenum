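; Hex tile actor for the map editor, with its mesh looked up by row name in DT_HexTable and its Z position set from a height level.
; Clicking the tile reports its IndexXY to BP_EditorController.
; Six border meshes show walls sized by a height difference of one to three, with inverse variants mapping an index to the opposite side.
; It also sums HCost and GCost for pathfinding and can switch to a path mesh.
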(event OnClicked(HexMesh)
  (params (TouchedComponent :type Primitive%20Component%20Object%20Reference) (ButtonPressed :type Key%20Structure :default "None"))
  ;[1 1 1] Select hex
  (bind _asbp_editor_controller (Utilities|Casting|CastToBP_EditorController (Game|GetPlayerController 0)))
  (Default|SelectHex _asbp_editor_controller (Variables|MapGeneration&Path|GetIndexXY)))

(event Custom|HexCostCalculate
  ;[1 1 1] Hex cost
  (Variables|MapGeneration&Path|SetHexCost (+ (Variables|MapGeneration&Path|GetHCost) (Variables|MapGeneration&Path|GetGCost))))

(event Custom|ChangeHeight
  (params (Height :type Integer))
  (bind _returnvalue (Transformation|GetActorLocation))
  ;[1 1 1] Change Height
  (Variables|Default|SetHeight Height)
  (Variables|Default|SetHeightZ (Math|Conversions|ToFloat(Integer) (* (Variables|Default|GetHeight) 7)))
  (Transformation|SetActorLocation (Math|Vector|MakeVector (.x _returnvalue) (.y _returnvalue) (Variables|Default|GetHeightZ)) false false))

(event Custom|RefreshHex
  (bind _returnvalue (Transformation|GetActorLocation))
  ;[1 1 1] Refresh hex
  (bind _returnvalue_2 (Utilities|GetDataTableRow "/Game/Map/MapData/DT_HexTable.DT_HexTable" (Variables|Default|GetHexName))
    (:then
      (bind _output_get (Variables|Default|SetHexStr _returnvalue_2))
      (Components|StaticMesh|SetStaticMesh (Variables|Default|GetHexMesh) (.mesh _output_get))
      (Variables|Default|SetHeightZ (Math|Conversions|ToFloat(Integer) (* (Variables|Default|GetHeight) 7)))
      (Transformation|SetActorLocation (Math|Vector|MakeVector (.x _returnvalue) (.y _returnvalue) (Variables|Default|GetHeightZ)) false false))))

(event Custom|ChangeHexSelect
  (params (StringName :type String))
  ;[1 1 1] Change hex
  (bind _output_get (Variables|Default|SetHexName (Utilities|String|StringToName StringName)))
  (bind _returnvalue (Utilities|GetDataTableRow "/Game/Map/MapData/DT_HexTable.DT_HexTable" _output_get)
    (:then
      (bind _output_get_2 (Variables|Default|SetHexStr _returnvalue))
      (Components|StaticMesh|SetStaticMesh (Variables|Default|GetHexMesh) (.mesh _output_get_2)))))

(event Custom|SpawnNearBorder
  (params (NeighbourIndex :type Integer) (HeightDif :type Integer))
  ;[1 1 1] Spawn Borders
  (switch int HeightDif
    (:1
      (CallFunction|SetBorderInverse NeighbourIndex "/Game/Map/Borders/Wall1.Wall1"))
    (:2
      (CallFunction|SetBorderInverse NeighbourIndex "/Game/Map/Borders/Wall2.Wall2"))
    (:3
      (CallFunction|SetBorderInverse NeighbourIndex "/Game/Map/Borders/Wall3.Wall3"))))

(event Custom|DestroyBorder
  (params (BorderIndex :type Integer) (InverseBorder? :type Boolean))
  ;[1 1 1] Correct borders
  (if InverseBorder?
    (switch int BorderIndex
      (:0
        (Components|StaticMesh|SetStaticMesh (Variables|Default|GetBorderMesh4) 0))
      (:1
        (Components|StaticMesh|SetStaticMesh (Variables|Default|GetBorderMesh5) 0))
      (:2
        (Components|StaticMesh|SetStaticMesh (Variables|Default|GetBorderMesh6) 0))
      (:3
        (Components|StaticMesh|SetStaticMesh (Variables|Default|GetBorderMesh1) 0))
      (:4
        (Components|StaticMesh|SetStaticMesh (Variables|Default|GetBorderMesh2) 0))
      (:5
        (Components|StaticMesh|SetStaticMesh (Variables|Default|GetBorderMesh3) 0)))
    (else
      (switch int BorderIndex
        (:0
          (Components|StaticMesh|SetStaticMesh (Variables|Default|GetBorderMesh1) 0))
        (:1
          (Components|StaticMesh|SetStaticMesh (Variables|Default|GetBorderMesh2) 0))
        (:2
          (Components|StaticMesh|SetStaticMesh (Variables|Default|GetBorderMesh3) 0))
        (:3
          (Components|StaticMesh|SetStaticMesh (Variables|Default|GetBorderMesh4) 0))
        (:4
          (Components|StaticMesh|SetStaticMesh (Variables|Default|GetBorderMesh5) 0))
        (:5
          (Components|StaticMesh|SetStaticMesh (Variables|Default|GetBorderMesh6) 0))))))

(event Custom|ChangeHexManual
  (params (NewName :type Text))
  ;[1 1 1] Change hex
  (bind _output_get (Variables|Default|SetHexName (Utilities|String|StringToName (Utilities|String|ToString(Text) NewName))))
  (bind _returnvalue (Utilities|GetDataTableRow "/Game/Map/MapData/DT_HexTable.DT_HexTable" _output_get)
    (:then
      (bind _output_get_2 (Variables|Default|SetHexStr _returnvalue))
      (Components|StaticMesh|SetStaticMesh (Variables|Default|GetHexMesh) (.mesh _output_get_2)))))

(event Custom|HexPath
  ;[1 1 1] Hex is part of path
  (Components|StaticMesh|SetStaticMesh (Variables|Default|GetHexMesh) "/Game/Map/Hexes/Meshes/Hex_Path.Hex_Path"))

(event Custom|SpawnSelfBorder
  (params (NeighbourIndex :type Integer) (HeightDif :type Integer))
  ;[1 1 1] Spawn Borders
  (switch int HeightDif
    (:1
      (CallFunction|SetBorderMesh NeighbourIndex "/Game/Map/Borders/Wall1.Wall1"))
    (:2
      (CallFunction|SetBorderMesh NeighbourIndex "/Game/Map/Borders/Wall2.Wall2"))
    (:3
      (CallFunction|SetBorderMesh NeighbourIndex "/Game/Map/Borders/Wall3.Wall3"))))

(event EventBeginPlay
  ;[1 1 1] Begin play
  (bind _returnvalue (Utilities|GetDataTableRow "/Game/Map/MapData/DT_HexTable.DT_HexTable" (Variables|Default|GetHexName))
    (:then
      (Variables|Default|SetHexStr _returnvalue))))

(fn ConstructionScript)

(fn SetBorderMesh
  (params (Index :type Integer) (StaticMesh :type Static%20Mesh%20Object%20Reference))
  (LocalVariables|Setl_Mesh StaticMesh)
  (switch int Index
    (:0
      (Components|StaticMesh|SetStaticMesh (Variables|Default|GetBorderMesh1) (LocalVariables|Getl_Mesh)))
    (:1
      (Components|StaticMesh|SetStaticMesh (Variables|Default|GetBorderMesh2) (LocalVariables|Getl_Mesh)))
    (:2
      (Components|StaticMesh|SetStaticMesh (Variables|Default|GetBorderMesh3) (LocalVariables|Getl_Mesh)))
    (:3
      (Components|StaticMesh|SetStaticMesh (Variables|Default|GetBorderMesh4) (LocalVariables|Getl_Mesh)))
    (:4
      (Components|StaticMesh|SetStaticMesh (Variables|Default|GetBorderMesh5) (LocalVariables|Getl_Mesh)))
    (:5
      (Components|StaticMesh|SetStaticMesh (Variables|Default|GetBorderMesh6) (LocalVariables|Getl_Mesh)))))

(fn SetBorderInverse
  (params (Index :type Integer) (StaticMesh :type Static%20Mesh%20Object%20Reference))
  (LocalVariables|Setl_Mesh StaticMesh)
  (switch int Index
    (:0
      (Components|StaticMesh|SetStaticMesh (Variables|Default|GetBorderMesh4) (LocalVariables|Getl_Mesh)))
    (:1
      (Components|StaticMesh|SetStaticMesh (Variables|Default|GetBorderMesh5) (LocalVariables|Getl_Mesh)))
    (:2
      (Components|StaticMesh|SetStaticMesh (Variables|Default|GetBorderMesh6) (LocalVariables|Getl_Mesh)))
    (:3
      (Components|StaticMesh|SetStaticMesh (Variables|Default|GetBorderMesh1) (LocalVariables|Getl_Mesh)))
    (:4
      (Components|StaticMesh|SetStaticMesh (Variables|Default|GetBorderMesh2) (LocalVariables|Getl_Mesh)))
    (:5
      (Components|StaticMesh|SetStaticMesh (Variables|Default|GetBorderMesh3) (LocalVariables|Getl_Mesh)))))