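; BP_Camera is a player-controlled free camera that pans and turns through axis input.
; MoveForward follows the actor's forward vector with Z zeroed, while MoveRight follows the Camera component's right vector, both scaled by CameraSpeed.
; RotationRight adds its axis value directly to actor yaw, preserving pitch and roll.
; Moves set the location without sweep, and neither movement nor rotation scales by delta time.
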(event Input|AxisEvents|InputAxisMoveRight
  (params (AxisValue :type Float%20%28single-precision%29))
  (Transformation|SetActorLocation (+ (* (Math|Vector|GetRightVector (Variables|Default|GetCamera)) (* (* AxisValue 2.0) (Variables|Default|GetCameraSpeed))) (Transformation|GetActorLocation)) false false))

(event Input|AxisEvents|InputAxisMoveForward
  (params (AxisValue :type Float%20%28single-precision%29))
  (bind _returnvalue (Transformation|GetActorForwardVector))
  (Transformation|SetActorLocation (+ (* (Math|Vector|MakeVector (.x _returnvalue) (.y _returnvalue) 0.0) (* (* AxisValue 2.0) (Variables|Default|GetCameraSpeed))) (Transformation|GetActorLocation)) false false))

(event Input|AxisEvents|InputAxisRotationRight
  (params (AxisValue :type Float%20%28single-precision%29))
  (bind _returnvalue (Transformation|GetActorRotation))
  (Transformation|SetActorRotation (Math|Rotator|MakeRotator (.roll _returnvalue) (.pitch _returnvalue) (+ AxisValue (.yaw _returnvalue)))))

(fn ConstructionScript)