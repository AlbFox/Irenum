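; Player controller for the hex map editor that spawns and possesses a camera pawn and shows the editor HUD.
; Selecting a hex pushes its coordinates, name and height to the HUD, while edit events change height or type and refresh the map's paths.
; Height edits also rebuild border pieces against the six neighbours, using column-parity offsets and height differences to spawn or destroy borders.
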(event Custom|SelectHex
  (params (VectorXY :type Vector%202D%20Structure))
  (bind _w_editorhud (Variables|Default|GetW_EditorHUD))
  ;[1 1 1] Select hex to edit
  (bind _output_get (Variables|/Game/Map/Editor/EditorInterface/W_EditorHUD.W_EditorHUD_C|SetVectorXY (Variables|Default|GetW_EditorHUD) VectorXY))
  (Variables|/Game/Map/Editor/EditorInterface/W_EditorHUD.W_EditorHUD_C|SetHexID _w_editorhud (Variables|/Game/Map/Hexes/BP_Hex.BP_Hex_C|GetHexName (.Value (Utilities|Map|Find (Variables|Default|GetHexMap) _output_get))))
  (Variables|/Game/Map/Editor/EditorInterface/W_EditorHUD.W_EditorHUD_C|SetHeight _w_editorhud (Variables|/Game/Map/Hexes/BP_Hex.BP_Hex_C|GetHeight (.Value (Utilities|Map|Find (Variables|Default|GetHexMap) _output_get))))
  (Default|HexSelected _w_editorhud))

(event Custom|EditHeight
  (params (NewHeight :type Integer) (HexXY :type Vector%202D%20Structure))
  (bind _hexmap (Variables|Default|GetHexMap))
  (bind _value (Utilities|Map|Find _hexmap HexXY))
  ;[1 1 1] Edit Height
  (bind _output_get (Variables|/Game/Map/Hexes/BP_Hex.BP_Hex_C|SetHeight _value NewHeight))
  (Default|ChangeHeight _value _output_get)
  (CallFunction|SetHexBorders HexXY)
  ;[1 1 1] Edit hex
  (Default|RefreshPath (Variables|Default|GetEditingMap)))

(event Custom|EditHexSelect
  (params (StringName :type String) (HexXY :type Vector%202D%20Structure))
  ;[1 1 1] Edit hex
  (Default|ChangeHexSelect (.Value (Utilities|Map|Find (Variables|Default|GetHexMap) HexXY)) StringName)
  (Default|RefreshPath (Variables|Default|GetEditingMap)))

(event Custom|EditHexManual
  (params (NewTypeName :type Text) (HexXY :type Vector%202D%20Structure))
  ;[1 1 1] Edit hex
  (Default|ChangeHexManual (.Value (Utilities|Map|Find (Variables|Default|GetHexMap) HexXY)) NewTypeName)
  (Default|RefreshPath (Variables|Default|GetEditingMap)))

(event EventBeginPlay
  ;[1 1 1] Begin play
  (Utilities|FlowControl|Sequence
    (:then_0
      (bind _returnvalue (Game|SpawnActorfromClass "/Game/Map/ModeCameraController/BP_Camera.BP_Camera_C" (Math|Transform|MakeTransform "0,400.000000,700.000000" "-60.000000,20.000000,0.000000" "1,1,1") "Undefined" 0 0))
      (bind _output_get (Variables|Default|SetPlayerCamera _returnvalue))
      (Pawn|Possess _output_get))
    (:then_1
      (bind _returnvalue_2 (UserInterface|CreateWidget "/Game/Map/Editor/EditorInterface/W_EditorHUD.W_EditorHUD_C" 0 self))
      (bind _output_get_2 (Variables|Default|SetW_EditorHUD _returnvalue_2))
      (UserInterface|Viewport|AddtoViewport _output_get_2 0))))

(fn ConstructionScript)

(fn SetHexBorders
  (params (HexXY :type Vector%202D%20Structure%20%28by%20ref%29))
  (bind _hexmap (Variables|Default|GetHexMap))
  (LocalVariables|Setl_Hex HexXY)
  (for (_array_element _array_index) (select (or (== (Math|Float|%(Float) (.x (LocalVariables|Getl_Hex)) 2.0) 0.0) (== (.x (LocalVariables|Getl_Hex)) 0.0)) (Utilities|Array|MakeArray "(X=1.000000,Y=0.000000)" "(X=1.000000,Y=-1.000000)" "(X=0.000000,Y=-1.000000)" "(X=-1.000000,Y=-1.000000)" "(X=-1.000000,Y=0.000000)" "(X=0.000000,Y=1.000000)") (Utilities|Array|MakeArray "(X=1.000000,Y=1.000000)" "(X=1.000000,Y=0.000000)" "(X=0.000000,Y=-1.000000)" "(X=-1.000000,Y=0.000000)" "(X=-1.000000,Y=1.000000)" "(X=0.000000,Y=1.000000)"))
    (LocalVariables|Setl_NeighbourIndex _array_index)
    (LocalVariables|Setl_Neighbour (+ _array_element (LocalVariables|Getl_Hex)))
    (if (.ReturnValue (Utilities|Map|Find _hexmap (+ _array_element (LocalVariables|Getl_Hex))))
      (if (== (- (Variables|/Game/Map/Hexes/BP_Hex.BP_Hex_C|GetHeight (.Value (Utilities|Map|Find _hexmap (+ _array_element (LocalVariables|Getl_Hex))))) (Variables|/Game/Map/Hexes/BP_Hex.BP_Hex_C|GetHeight (.Value (Utilities|Map|Find _hexmap (LocalVariables|Getl_Hex))))) 0)
        (Default|DestroyBorder (.Value (Utilities|Map|Find (Variables|Default|GetHexMap) (LocalVariables|Getl_Hex))) (LocalVariables|Getl_NeighbourIndex) false)
        (Default|DestroyBorder (.Value (Utilities|Map|Find (Variables|Default|GetHexMap) (LocalVariables|Getl_Neighbour))) (LocalVariables|Getl_NeighbourIndex) true)
        (else
          (LocalVariables|Setl_HeightDif (Math|Integer|Absolute(Integer) (- (Variables|/Game/Map/Hexes/BP_Hex.BP_Hex_C|GetHeight (.Value (Utilities|Map|Find _hexmap (+ _array_element (LocalVariables|Getl_Hex))))) (Variables|/Game/Map/Hexes/BP_Hex.BP_Hex_C|GetHeight (.Value (Utilities|Map|Find _hexmap (LocalVariables|Getl_Hex)))))))
          (if (> (- (Variables|/Game/Map/Hexes/BP_Hex.BP_Hex_C|GetHeight (.Value (Utilities|Map|Find _hexmap (+ _array_element (LocalVariables|Getl_Hex))))) (Variables|/Game/Map/Hexes/BP_Hex.BP_Hex_C|GetHeight (.Value (Utilities|Map|Find _hexmap (LocalVariables|Getl_Hex))))) 0)
            (Default|DestroyBorder (.Value (Utilities|Map|Find (Variables|Default|GetHexMap) (LocalVariables|Getl_Neighbour))) (LocalVariables|Getl_NeighbourIndex) true)
            (Default|SpawnSelfBorder (.Value (Utilities|Map|Find (Variables|Default|GetHexMap) (LocalVariables|Getl_Hex))) (LocalVariables|Getl_NeighbourIndex) (LocalVariables|Getl_HeightDif))
            (else
              (Default|DestroyBorder (.Value (Utilities|Map|Find (Variables|Default|GetHexMap) (LocalVariables|Getl_Hex))) (LocalVariables|Getl_NeighbourIndex) false)
              (Default|SpawnNearBorder (.Value (Utilities|Map|Find (Variables|Default|GetHexMap) (LocalVariables|Getl_Neighbour))) (LocalVariables|Getl_NeighbourIndex) (LocalVariables|Getl_HeightDif)))))))))